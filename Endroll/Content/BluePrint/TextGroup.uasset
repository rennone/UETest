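; TextGroup is an actor Blueprint that is mostly a stub, with nothing in the file showing how it groups text.
; BeginPlay binds a handler to its own OnDestroyed event, but that handler, Tick, the construction script and the Update function are all empty.
; Unconnected leftover nodes print the DefaultSceneRoot1 location and attempt to delete all children by looping DestroyActor while child components remain.
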(event `self.ReceiveBeginPlay`
  (add `self.OnDestroyed` (delegate `OnDestroyed_イベント_0`)))

(event `OnDestroyed_イベント_0`)

(event `self.ReceiveTick`
  (params (DeltaSeconds :type "Float (single-precision)")))

(fn `Update`)

(fn `UserConstructionScript`)